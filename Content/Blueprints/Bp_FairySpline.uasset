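; Spline path actor that moves the level's Bp_TempFairy along its spline.
; BeginPlay finds and caches the fairy with GetActorOfClass.
; The FollowSpline event plays the UpdateLocation timeline at a rate of one over Duration, lerping its Alpha across the spline length to set the fairy's world location and rotation.
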(event `self.ReceiveBeginPlay`
  (bind _returnvalue (`GameplayStatics.GetActorOfClass` "/Game/Blueprints/Bp_TempFairy.Bp_TempFairy_C"))
  (set `self.FairyRef` _returnvalue))

(event `FollowSpline`
  (bind _spline (`self.Spline`))
  (bind _returnvalue (`KismetMathLibrary.Lerp` 0.0 (`SplineComponent.GetSplineLength` _spline) (`self.Alpha`)))
  (`TimelineComponent.SetPlayRate` (`self.UpdateLocation`) (/ 1.0 (`self.Duration`)))
  (bind (_direction _alpha) (`Timeline|UpdateLocation`)
    (:`Update`
      (set `self.Alpha` _alpha)
      (`self.K2_SetActorLocationAndRotation` (`self.FairyRef`) (`SplineComponent.GetLocationAtDistanceAlongSpline` _spline _returnvalue "World") (`SplineComponent.GetRotationAtDistanceAlongSpline` _spline _returnvalue "World") false false))))

(fn `UserConstructionScript`)