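; BP_Camera is a follow camera that trails the BP_Dent actor from a fixed offset behind it on world X and slightly above.
; BeginPlay finds and stores the BP_Dent instance as its target.
; Each Tick eases the Camera component toward the offset position with VInterpTo.
; The offset is in world axes, so the camera does not follow the target's rotation.
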(event `self.ReceiveBeginPlay`
  (bind _returnvalue (`GameplayStatics.GetActorOfClass` "/Game/Blueprints/Player/BP_Dent.BP_Dent_C"))
  (set `self.target` _returnvalue))

(event `self.ReceiveTick`
  (params (DeltaSeconds :type "Float (single-precision)"))
  (bind _camera (`self.Camera`))
  (bind _returnvalue (`self.GetTransform` (`self.target`)))
  (`SceneComponent.K2_SetWorldTransform` _camera (`KismetMathLibrary.MakeTransform` (`KismetMathLibrary.VInterpTo` (`SceneComponent.K2_GetComponentLocation` _camera) (`KismetMathLibrary.MakeVector` (- (.x (.location _returnvalue)) 700.0) (.y (.location _returnvalue)) (+ (.z (.location _returnvalue)) 150.0)) DeltaSeconds 10.0)) false false))

(fn `UserConstructionScript`)