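; Trigger volume that slows the spline-following fairy when the player character enters it.
; On the first player overlap of its collision component, it lengthens the referenced fairy's Duration by a multiplier.
; It then sets the play rate of the fairy's UpdateLocation timeline to the inverse of the new duration.
; A DoOnce gate limits the slowdown to a single use per trigger.
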(event `self.CollisionComponent.OnComponentBeginOverlap`
  (params (OverlappedComponent :type "PrimitiveComponent Object Reference") (OtherActor :type "Actor Object Reference") (OtherComp :type "PrimitiveComponent Object Reference") (OtherBodyIndex :type Integer) (bFromSweep :type Boolean) (SweepResult :type "HitResult Structure (by ref)"))
  (bind _splinefairyref (`self.SplineFairyRef`))
  (if (== OtherActor (`GameplayStatics.GetPlayerCharacter` 0))
    (`/Engine/EditorBlueprintResources/StandardMacros.DoOnce` false
      (:`Completed`
        (bind _output_get (set `/Game/Blueprints/Bp_FairySpline.Duration` (* (`/Game/Blueprints/Bp_FairySpline.Duration` _splinefairyref) 1.3) _splinefairyref))
        (`TimelineComponent.SetPlayRate` (`/Game/Blueprints/Bp_FairySpline.UpdateLocation` _splinefairyref) (/ 1.0 _output_get))))))

(fn `UserConstructionScript`)