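; BP_Window is a window hazard that periodically opens, throws a random object along a spline, then closes.
; A looping timer starts a chain of timelines that swings both panes open by yaw, moves the object along the spline, then swings the panes shut.
; Each launch picks a random mesh, and the object returns to the spline start afterward.
; Any BP_Dent, BP_Strong or BP_Agile it overlaps is destroyed.
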(event `self.ReceiveBeginPlay`
  (bind (_relativerotation_roll _relativerotation_pitch _relativerotation_yaw) (`KismetMathLibrary.BreakRotator` (`SceneComponent.RelativeRotation` (`self.SM_WindowTestLeft`))))
  (bind (_relativerotation_roll_2 _relativerotation_pitch_2 _relativerotation_yaw_2) (`KismetMathLibrary.BreakRotator` (`SceneComponent.RelativeRotation` (`self.SM_WindowTestRight`))))
  (`TimelineComponent.SetPlayRate` (`self.Open_Window`) 2.0)
  (`TimelineComponent.SetPlayRate` (`self.Timeline_0`) 2.0)
  (`TimelineComponent.SetPlayRate` (`self.MoveAlongSpline`) 0.65)
  (set `self.LeftWindowRotation` _relativerotation_yaw)
  (set `self.RightWindowRotation` _relativerotation_yaw_2)
  (`self.OpenWindow`)
  (`KismetSystemLibrary.K2_SetTimerDelegate` (delegate `OpenWindow`) 5.0 true))

(event `OpenWindow`
  (bind (_direction _movment) (`Timeline|Open_Window` :!via `PlayFromStart`)
    (:`Update`
      (bind _returnvalue (* _movment (`self.RotationDistance`)))
      (`SceneComponent.K2_SetRelativeRotation` (`self.SM_WindowTestLeft`) (`KismetMathLibrary.MakeRotator` 0.0 0.0 (+ _returnvalue (`self.LeftWindowRotation`))) false false)
      (`SceneComponent.K2_SetRelativeRotation` (`self.SM_WindowTestRight`) (`KismetMathLibrary.MakeRotator` 0.0 0.0 (- (`self.RightWindowRotation`) _returnvalue)) false false))
    (:`Finished`
      (`KismetSystemLibrary.Delay` 1.0)
      (`self.LaunchObject`))))

(event `LaunchObject`
  (bind _returnvalue (`KismetMathLibrary.Lerp` 0.0 (`SplineComponent.GetSplineLength` (`self.ObjectSpline`)) (`self.Alpha`)))
  (`StaticMeshComponent.SetStaticMesh` (`self.LaunchedObject`) (`KismetArrayLibrary.Array_Random` (`self.RandomObject`)))
  (bind (_direction _speed) (`Timeline|MoveAlongSpline` :!via `PlayFromStart`)
    (:`Update`
      (set `self.Alpha` _speed)
      (`SceneComponent.K2_SetWorldLocationAndRotation` (`self.LaunchedObject`) (`SplineComponent.GetLocationAtDistanceAlongSpline` (`self.ObjectSpline`) _returnvalue "World") (`SplineComponent.GetRotationAtDistanceAlongSpline` (`self.ObjectSpline`) _returnvalue "World") false false))
    (:`Finished`
      (bind (_direction_2 _movment) (`Timeline|Timeline_0` :!via `ReverseFromEnd`)
        (:`Update`
          (bind _returnvalue_2 (* _movment (`self.RotationDistance`)))
          (`SceneComponent.K2_SetRelativeRotation` (`self.SM_WindowTestLeft`) (`KismetMathLibrary.MakeRotator` 0.0 0.0 (+ _returnvalue_2 (`self.LeftWindowRotation`))) false false)
          (`SceneComponent.K2_SetRelativeRotation` (`self.SM_WindowTestRight`) (`KismetMathLibrary.MakeRotator` 0.0 0.0 (- (`self.RightWindowRotation`) _returnvalue_2)) false false))
        (:`Finished`
          (`SceneComponent.K2_SetWorldLocation` (`self.LaunchedObject`) (`SplineComponent.GetLocationAtSplinePoint` (`self.ObjectSpline`) 0 "World") false false))))))

(event `self.LaunchedObject.OnComponentBeginOverlap`
  (params (OverlappedComponent :type "PrimitiveComponent Object Reference") (OtherActor :type "Actor Object Reference") (OtherComp :type "PrimitiveComponent Object Reference") (OtherBodyIndex :type Integer) (bFromSweep :type Boolean) (SweepResult :type "HitResult Structure (by ref)"))
  (bind _asbp_dent (cast `/Game/Blueprints/Player/BP_Dent` OtherActor)
    (:`then`
      (`self.K2_DestroyActor` _asbp_dent))
    (:`CastFailed`
      (bind _asbp_strong (cast `/Game/Blueprints/Player/BP_Strong` OtherActor)
        (:`then`
          (`self.K2_DestroyActor` _asbp_strong))
        (:`CastFailed`
          (bind _asbp_agile (cast `/Game/Blueprints/Player/BP_Agile` OtherActor))
          (`self.K2_DestroyActor` _asbp_agile))))))

(fn `UserConstructionScript`)