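; Destructible cube actor that loses health from any damage and shatters when health reaches zero.
; Its Destruct event applies one point of damage to itself, feeding the same damage handler.
; On breaking, it plays a sound, swaps the cube and widget for a geometry collection, and spawns a master field with a camera shake.
; The box collider is removed and debris collision disabled before the actor destroys itself after a short delay.
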(event `self.ReceiveAnyDamage`
  (params (Damage :type "Float (single-precision)") (DamageType :type "DamageType Object Reference") (InstigatedBy :type "Controller Object Reference") (DamageCauser :type "Actor Object Reference"))
  (bind _shape_cube_geometrycollection (`self.Shape_Cube_GeometryCollection`))
  (bind _output_get (set `self.Health` (`KismetMathLibrary.FClamp` (- (`self.Health`) Damage) 0.0 (`self.HealthMax`))))
  (if (== _output_get 0.0)
    (`GameplayStatics.PlaySound2D` "/Game/Assets/SFX/Sc_BreakWall.Sc_BreakWall" 1.0 1.0 0.0 null null)
    (`SceneComponent.SetVisibility` (`self.Shape_Cube_GeometryCollection`) true false)
    (bind _box (`self.Box`)
      (:`then`
        (`ActorComponent.K2_DestroyComponent` _box)
        (`SceneComponent.SetVisibility` (`self.Cube`) false false)
        (`SceneComponent.SetVisibility` (`self.Widget`) false false)
        (`|SpawnActorFromClass` "/Engine/EditorResources/FieldNodes/FS_MasterField.FS_MasterField_C" (`self.GetTransform`) "AlwaysSpawn" "OverrideRootScale" null null)
        (`GameplayStatics.PlayWorldCameraShake` "/Game/Blueprints/Bp_CameraShake.Bp_CameraShake_C" (`SceneComponent.K2_GetComponentLocation` (`Character.Mesh` (`GameplayStatics.GetPlayerCharacter` 0))) 0.0 800.0)
        (`PrimitiveComponent.SetCollisionResponseToChannel` _shape_cube_geometrycollection "ECC_Pawn" "ECR_Ignore")
        (`PrimitiveComponent.SetCollisionEnabled` _shape_cube_geometrycollection "NoCollision")
        (`KismetSystemLibrary.Delay` 2.0)
        (`self.K2_DestroyActor`))
      (:`else`))))

(event `/Game/Blueprints/BPI_Destructible.Destruct`
  (params (StrongRef :type "/Game/Blueprints/Player/BP_Strong Object Reference"))
  (`GameplayStatics.ApplyDamage` self 1.0 null StrongRef))

(fn `UserConstructionScript`)