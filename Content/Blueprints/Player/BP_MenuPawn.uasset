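; Menu pawn that moves itself on the Y/Z plane in response to the gamepad right stick.
; GamepadRight2D offsets and scales the axis to viewport size, then clamps and remaps it to a screen-centered position with vertical inverted, so half deflection reaches the edge.
; A similar mouse-position path exists but is disconnected, leaving Mouse2D empty.
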(event `self.ReceiveTick`
  (params (DeltaSeconds :type "Float (single-precision)")))

(event `InputVectorAxis|Mouse2D`
  (params (AxisValue :type "Vector Structure")))

(event `InputVectorAxis|Gamepad_Right2D`
  (params (AxisValue :type "Vector Structure"))
  (bind (_returnvalue_x _returnvalue_y) (`KismetMathLibrary.BreakVector2D` (`WidgetLayoutLibrary.GetViewportSize`)))
  (bind _returnvalue (/ _returnvalue_x 2.0))
  (bind _returnvalue_2 (/ _returnvalue_y 2.0))
  (`self.K2_SetActorLocation` (`KismetMathLibrary.MakeVector` 0.0 (`KismetMathLibrary.MapRangeClamped` (* (+ (.x AxisValue) 0.5) _returnvalue_x) 0.0 _returnvalue_x (- 0.0 _returnvalue) _returnvalue) (- 0.0 (`KismetMathLibrary.MapRangeClamped` (* (+ (.y AxisValue) 0.5) _returnvalue_y) 0.0 _returnvalue_y (- 0.0 _returnvalue_2) _returnvalue_2) 0.0))))

(fn `UserConstructionScript`)