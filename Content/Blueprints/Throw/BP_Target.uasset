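; BP_Target is a lockable target for the throw system.
; Lock shows its ThrowWidget component, sets IsLock and writes itself into the instigator's Target reference.
; Unlock hides the widget, clears IsLock and sets the instigator's Target to None.
; Helper functions wrap the widget's visibility, including a getter for its current state.
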(event `self.ReceiveBeginPlay`)

(event `/Game/Blueprints/Throw/BPI_Throw.Lock`
  (params (Instigator :type "/Game/Blueprints/Player/BP_Strong Object Reference"))
  (`self.ShowWidget`)
  (set `self.isLock` true)
  (set `/Game/Blueprints/Player/BP_Strong.Target` self Instigator))

(event `/Game/Blueprints/Throw/BPI_Throw.Unlock`
  (params (Instigator :type "/Game/Blueprints/Player/BP_Strong Object Reference"))
  (`self.HideWidget`)
  (set `self.isLock` false)
  (set `/Game/Blueprints/Player/BP_Strong.Target` null Instigator))

(fn `GetWidgetVisibility`
  (returns (Visible :type Boolean))
  (return (`SceneComponent.bVisible` (`self.ThrowWidget`))))

(fn `HideWidget`
  (`SceneComponent.SetVisibility` (`self.ThrowWidget`) false false))

(fn `ShowWidget`
  (`SceneComponent.SetVisibility` (`self.ThrowWidget`) true false))

(fn `UserConstructionScript`)