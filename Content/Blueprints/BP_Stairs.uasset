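; Stairs actor that automatically carries a BP_Dent or BP_Strong character along a spline when it enters the overlap volume.
; On overlap it stores the character, disables its movement and plays a shared timeline.
; The timeline alpha maps to distance along StairsSpline, setting location and yaw for every stored character, then restores Walking when finished.
; The timeline is never reversed or reset, and stored references are never cleared.
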(event `self.Overlapp.OnComponentBeginOverlap`
  (params (OverlappedComponent :type "PrimitiveComponent Object Reference") (OtherActor :type "Actor Object Reference") (OtherComp :type "PrimitiveComponent Object Reference") (OtherBodyIndex :type Integer) (bFromSweep :type Boolean) (SweepResult :type "HitResult Structure (by ref)"))
  (bind _returnvalue (`KismetMathLibrary.Lerp` 0.0 (`SplineComponent.GetSplineLength` (`self.StairsSpline`)) (`self.Alpha`)))
  (bind _returnvalue_2 (`SplineComponent.GetLocationAtDistanceAlongSpline` (`self.StairsSpline`) _returnvalue "World"))
  (bind (_returnvalue_roll _returnvalue_pitch _returnvalue_yaw) (`KismetMathLibrary.BreakRotator` (`SplineComponent.GetRotationAtDistanceAlongSpline` (`self.StairsSpline`) _returnvalue "World")))
  (bind _asbp_dent (cast `/Game/Blueprints/Player/BP_Dent` OtherActor)
    (:`then`
      (set `self.As BP Dent` _asbp_dent)
      (`CharacterMovementComponent.DisableMovement` (`Character.CharacterMovement` _asbp_dent))
      (bind (_direction _newtrack_0) (`Timeline|Timeline_0` :!label _label)
        (:`Update`
          (set `self.Alpha` _newtrack_0)
          (`|ExecutionSequence`
            (:`then_0`
              (bind _as_bp_dent (`self.As BP Dent`)
                (:`then`
                  (`self.K2_SetActorLocationAndRotation` _as_bp_dent _returnvalue_2 (`KismetMathLibrary.MakeRotator` 0.0 0.0 _returnvalue_yaw) false false))
                (:`else`)))
            (:`then_1`
              (bind _as_bp_strong (`self.As BP Strong`)
                (:`then`
                  (`self.K2_SetActorLocationAndRotation` _as_bp_strong _returnvalue_2 (`KismetMathLibrary.MakeRotator` 0.0 0.0 _returnvalue_yaw) false false))
                (:`else`)))))
        (:`Finished`
          (`|ExecutionSequence`
            (:`then_0`
              (bind _as_bp_dent_2 (`self.As BP Dent`)
                (:`then`
                  (`CharacterMovementComponent.SetMovementMode` (`Character.CharacterMovement` _as_bp_dent_2) "MOVE_Walking" 0))
                (:`else`)))
            (:`then_1`
              (bind _as_bp_strong_2 (`self.As BP Strong`)
                (:`then`
                  (`CharacterMovementComponent.SetMovementMode` (`Character.CharacterMovement` _as_bp_strong_2) "MOVE_Walking" 0))
                (:`else`)))))))
    (:`CastFailed`
      (bind _asbp_strong (cast `/Game/Blueprints/Player/BP_Strong` OtherActor))
      (set `self.As BP Strong` _asbp_strong)
      (`CharacterMovementComponent.DisableMovement` (`Character.CharacterMovement` _asbp_strong))
      (goto _label))))

(fn `UserConstructionScript`)