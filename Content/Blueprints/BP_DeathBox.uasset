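; BP_DeathBox is a kill volume that ends the game when the player character enters its Box.
; The overlap event adds a WBP_GameOver widget to the viewport and disables the player's input.
; Tick also polls the Box's overlapping characters and runs the same response through a DoOnce.
; The overlap path is not gated by that DoOnce, so both paths can each create a widget.
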(event `self.Box.OnComponentBeginOverlap`
  (params (OverlappedComponent :type "PrimitiveComponent Object Reference") (OtherActor :type "Actor Object Reference") (OtherComp :type "PrimitiveComponent Object Reference") (OtherBodyIndex :type Integer) (bFromSweep :type Boolean) (SweepResult :type "HitResult Structure (by ref)"))
  (bind _returnvalue (`GameplayStatics.GetPlayerCharacter` 0))
  (if (== OtherActor _returnvalue)
    (bind _returnvalue_2 (`|CreateWidget` "/Game/UI/WBP_GameOver.WBP_GameOver_C"))
    (`UserWidget.AddToViewport` _returnvalue_2 0)
    (`self.DisableInput` (`CharacterMovementComponent.GetCharacterOwner` (`Character.CharacterMovement` _returnvalue)) (`GameplayStatics.GetPlayerController` 0))))

(event `self.ReceiveTick`
  (params (DeltaSeconds :type "Float (single-precision)"))
  (bind _returnvalue (`GameplayStatics.GetPlayerCharacter` 0))
  (for _array_element (`PrimitiveComponent.GetOverlappingActors` (`self.Box`) "/Script/Engine.Character")
    (if (== _array_element _returnvalue)
      (`/Engine/EditorBlueprintResources/StandardMacros.DoOnce` false
        (:`Completed`
          (bind _returnvalue_2 (`|CreateWidget` "/Game/UI/WBP_GameOver.WBP_GameOver_C"))
          (`UserWidget.AddToViewport` _returnvalue_2 0)
          (`self.DisableInput` (`CharacterMovementComponent.GetCharacterOwner` (`Character.CharacterMovement` _returnvalue)) (`GameplayStatics.GetPlayerController` 0)))))))

(fn `UserConstructionScript`)