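; Building actor that swaps itself for a destructible version once three of its walls are destroyed.
; Tick polls the destroyed-wall count and, once, hides the actor, disables its collision and spawns Bp_DestrutibleBuilding at the same transform.
; The spawned geometry collections are set to ignore pawns and use query-only collision.
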(event `self.ReceiveTick`
  (params (DeltaSeconds :type "Float (single-precision)"))
  (bind (_returnvalue_location _returnvalue_rotation _returnvalue_scale) (`KismetMathLibrary.BreakTransform` (`self.GetTransform`)))
  (if (== (`self.NbrWallDestroy`) 3)
    (`/Engine/EditorBlueprintResources/StandardMacros.DoOnce` false
      (:`Completed`
        (`self.SetActorEnableCollision` false)
        (`self.SetActorHiddenInGame` true)
        (bind _returnvalue (`|SpawnActorFromClass` "/Game/Blueprints/Bp_DestrutibleBuilding.Bp_DestrutibleBuilding_C" (`KismetMathLibrary.MakeTransform` _returnvalue_location _returnvalue_rotation _returnvalue_scale) "AlwaysSpawn" "OverrideRootScale" null null))
        (bind _shape_cube348_geometrycollection (`/Game/Blueprints/Bp_DestrutibleBuilding.Shape_Cube348_GeometryCollection` _returnvalue))
        (`PrimitiveComponent.SetCollisionResponseToChannel` _shape_cube348_geometrycollection "ECC_Pawn" "ECR_Ignore")
        (`PrimitiveComponent.SetCollisionResponseToChannel` (`/Game/Blueprints/Bp_DestrutibleBuilding.SM_Maison_E_GeometryCollection` _returnvalue) "ECC_Pawn" "ECR_Ignore")
        (`PrimitiveComponent.SetCollisionResponseToChannel` (`/Game/Blueprints/Bp_DestrutibleBuilding.SM_Maison_E2_GeometryCollection` _returnvalue) "ECC_Pawn" "ECR_Ignore")
        (`PrimitiveComponent.SetCollisionResponseToChannel` (`/Game/Blueprints/Bp_DestrutibleBuilding.SM_Maison_F_GeometryCollection` _returnvalue) "ECC_Pawn" "ECR_Ignore")
        (`PrimitiveComponent.SetCollisionResponseToChannel` (`/Game/Blueprints/Bp_DestrutibleBuilding.SM_Maison_F2_GeometryCollection` _returnvalue) "ECC_Pawn" "ECR_Ignore")
        (`PrimitiveComponent.SetCollisionEnabled` _shape_cube348_geometrycollection "QueryOnly")
        (`PrimitiveComponent.SetCollisionEnabled` (`/Game/Blueprints/Bp_DestrutibleBuilding.SM_Maison_E_GeometryCollection` _returnvalue) "QueryOnly")
        (`PrimitiveComponent.SetCollisionEnabled` (`/Game/Blueprints/Bp_DestrutibleBuilding.SM_Maison_E2_GeometryCollection` _returnvalue) "QueryOnly")
        (`PrimitiveComponent.SetCollisionEnabled` (`/Game/Blueprints/Bp_DestrutibleBuilding.SM_Maison_F_GeometryCollection` _returnvalue) "QueryOnly")
        (`PrimitiveComponent.SetCollisionEnabled` (`/Game/Blueprints/Bp_DestrutibleBuilding.SM_Maison_F2_GeometryCollection` _returnvalue) "QueryOnly")))))

(fn `UserConstructionScript`)