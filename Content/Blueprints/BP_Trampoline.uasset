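; Trampoline actor that bounces characters upward when they overlap its collision box, with launches that vary by character and bounce count.
; A cast chain identifies BP_Dent, BP_Strong, BP_Agile or BP_TempTrampoline, each with its own three-tier vertical launch velocities selected by the character's NmbTrampo.
; After launching, it calls AddNmbTramp on the character, then plays a short, medium or strong sound selected by NmbTrampo read after that call.
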(event `self.CollisionBox.OnComponentBeginOverlap`
  (params (OverlappedComponent :type "PrimitiveComponent Object Reference") (OtherActor :type "Actor Object Reference") (OtherComp :type "PrimitiveComponent Object Reference") (OtherBodyIndex :type Integer) (bFromSweep :type Boolean) (SweepResult :type "HitResult Structure (by ref)"))
  (bind _asbp_dent (cast `/Game/Blueprints/Player/BP_Dent` OtherActor)
    (:`then`
      (bind _nmbtrampo (`/Game/Blueprints/Player/BP_Dent.NmbTrampo` _asbp_dent))
      (`Character.LaunchCharacter` _asbp_dent (`KismetMathLibrary.MakeVector` 0.0 0.0 (select `int` _nmbtrampo :`0` 300.0 :`1` 500.0 :`2` 800.0)) false true)
      (`/Game/Blueprints/Player/BP_Dent.AddNmbTramp` _asbp_dent)
      (`GameplayStatics.PlaySoundAtLocation` (select `int` _nmbtrampo :`0` "/Game/Assets/SFX/Trampoline/Short/SC_ShortTrampoline.SC_ShortTrampoline" :`1` "/Game/Assets/SFX/Trampoline/Medium/SC_MediumTrampoline.SC_MediumTrampoline" :`2` "/Game/Assets/SFX/Trampoline/Strong/SC_StrongTrampoline.SC_StrongTrampoline" :!type "SoundBase Object Reference") (`self.K2_GetActorLocation`) (struct) 1.0 1.0 0.0 null null null null))
    (:`CastFailed`
      (bind _asbp_strong (cast `/Game/Blueprints/Player/BP_Strong` OtherActor)
        (:`then`
          (bind _nmbtrampo_2 (`/Game/Blueprints/Player/BP_Strong.NmbTrampo` _asbp_strong))
          (`Character.LaunchCharacter` _asbp_strong (`KismetMathLibrary.MakeVector` 0.0 0.0 (select `int` _nmbtrampo_2 :`0` 300.0 :`1` 400.0 :`2` 600.0)) false true)
          (`/Game/Blueprints/Player/BP_Strong.AddNmbTramp` _asbp_strong)
          (`GameplayStatics.PlaySoundAtLocation` (select `int` _nmbtrampo_2 :`0` "/Game/Assets/SFX/Trampoline/Short/SC_ShortTrampoline.SC_ShortTrampoline" :`1` "/Game/Assets/SFX/Trampoline/Medium/SC_MediumTrampoline.SC_MediumTrampoline" :`2` "/Game/Assets/SFX/Trampoline/Strong/SC_StrongTrampoline.SC_StrongTrampoline" :!type "SoundBase Object Reference") (`self.K2_GetActorLocation`) (struct) 1.0 1.0 0.0 null null null null))
        (:`CastFailed`
          (bind _asbp_agile (cast `/Game/Blueprints/Player/BP_Agile` OtherActor)
            (:`then`
              (bind _nmbtrampo_3 (`/Game/Blueprints/Player/BP_Agile.NmbTrampo` _asbp_agile))
              (`Character.LaunchCharacter` _asbp_agile (`KismetMathLibrary.MakeVector` 0.0 0.0 (select `int` _nmbtrampo_3 :`0` 600.0 :`1` 900.0 :`2` 1200.0)) false true)
              (`/Game/Blueprints/Player/BP_Agile.AddNmbTramp` _asbp_agile)
              (`GameplayStatics.PlaySoundAtLocation` (select `int` _nmbtrampo_3 :`0` "/Game/Assets/SFX/Trampoline/Short/SC_ShortTrampoline.SC_ShortTrampoline" :`1` "/Game/Assets/SFX/Trampoline/Medium/SC_MediumTrampoline.SC_MediumTrampoline" :`2` "/Game/Assets/SFX/Trampoline/Strong/SC_StrongTrampoline.SC_StrongTrampoline" :!type "SoundBase Object Reference") (`self.K2_GetActorLocation`) (struct) 1.0 1.0 0.0 null null null null))
            (:`CastFailed`
              (bind _asbp_temp_trampoline (cast `/Game/Blueprints/Player/BP_TempTrampoline` OtherActor))
              (`Character.LaunchCharacter` _asbp_temp_trampoline (`KismetMathLibrary.MakeVector` 0.0 0.0 (select `int` (`/Game/Blueprints/Player/BP_TempTrampoline.NmbTrampo` _asbp_temp_trampoline) :`0` 500.0 :`1` 700.0 :`2` 900.0)) false true)
              (`/Game/Blueprints/Player/BP_TempTrampoline.AddNmbTramp` _asbp_temp_trampoline)
              (`GameplayStatics.PlaySoundAtLocation` (select `int` (`/Game/Blueprints/Player/BP_TempTrampoline.NmbTrampo` _asbp_temp_trampoline) :`0` "/Game/Assets/SFX/Trampoline/Short/SC_ShortTrampoline.SC_ShortTrampoline" :`1` "/Game/Assets/SFX/Trampoline/Medium/SC_MediumTrampoline.SC_MediumTrampoline" :`2` "/Game/Assets/SFX/Trampoline/Strong/SC_StrongTrampoline.SC_StrongTrampoline" :!type "SoundBase Object Reference") (`self.K2_GetActorLocation`) (struct) 1.0 1.0 0.0 null null null null))))))))

(fn `UserConstructionScript`)