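; Bp_Wall is a destructible wall with health, part of a building that tracks destroyed walls.
; Incoming damage lowers clamped health, and a Destruct event applies damage to itself.
; At zero health it increments the building's destroyed-wall count, spawns a Chaos field actor to break the geometry collection, turns off that collection's collision, removes the cube mesh and shakes the camera.
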(event `self.ReceiveAnyDamage`
  (params (Damage :type "Float (single-precision)") (DamageType :type "DamageType Object Reference") (InstigatedBy :type "Controller Object Reference") (DamageCauser :type "Actor Object Reference"))
  (bind _output_get (set `self.Health` (`KismetMathLibrary.FClamp` (- (`self.Health`) Damage) 0.0 (`self.HealthMax`))))
  (if (== _output_get 0.0)
    (`/Engine/EditorBlueprintResources/StandardMacros.IncrementInt` (`/Game/Blueprints/Bp_Buildings.NbrWallDestroy` (`self.BuildingRef`))
      (:`  `
        (`|SpawnActorFromClass` "/Engine/EditorResources/FieldNodes/FS_MasterField.FS_MasterField_C" (`self.GetTransform`) "AlwaysSpawn" "OverrideRootScale" null null)
        (`PrimitiveComponent.SetCollisionEnabled` (`self.Shape_Cube_GeometryCollection`) "NoCollision")
        (`ActorComponent.K2_DestroyComponent` (`self.Cube`))
        (`GameplayStatics.PlayWorldCameraShake` "/Game/Blueprints/Bp_CameraShake.Bp_CameraShake_C" (`SceneComponent.K2_GetComponentLocation` (`Character.Mesh` (`GameplayStatics.GetPlayerCharacter` 0))) 0.0 800.0)))))

(event `/Game/Blueprints/BPI_Destructible.Destruct`
  (params (StrongRef :type "/Game/Blueprints/Player/BP_Strong Object Reference"))
  (`GameplayStatics.ApplyDamage` self 2.0 null StrongRef))

(fn `UserConstructionScript`)