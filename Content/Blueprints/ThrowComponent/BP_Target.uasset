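; BP_Target is a target actor for the throw component that can be locked onto and shows a throw widget when locked.
; The Lock event makes its ThrowWidget visible and sets itself as the instigator's Target.
; Helper functions show, hide and query the widget's visibility, and BeginPlay prints the initial visibility state.
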(event `self.ReceiveBeginPlay`
  (`KismetSystemLibrary.PrintString` (`KismetStringLibrary.Conv_BoolToString` (`self.GetWidgetVisibility`))))

(event `/Game/Blueprints/ThrowComponent/BPI_Throw.Lock`
  (params (Instigator :type "/Game/Blueprints/Player/BP_Strong Object Reference"))
  (`self.ShowWidget`)
  (set `/Game/Blueprints/Player/BP_Strong.Target` self Instigator))

(fn `GetWidgetVisibility`
  (returns (Visible :type Boolean))
  (return (`SceneComponent.bVisible` (`self.ThrowWidget`))))

(fn `HideWidget`
  (`SceneComponent.SetVisibility` (`self.ThrowWidget`) false false))

(fn `ShowWidget`
  (`SceneComponent.SetVisibility` (`self.ThrowWidget`) true false))

(fn `UserConstructionScript`)